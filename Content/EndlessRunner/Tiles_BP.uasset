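; Endless-runner track tile that spawns obstacles on BeginPlay, with an independent one-in-three roll for each of its left, middle and right lanes.
; When the Runner overlaps its box, it asks RunnerGameMode to spawn the next tile and adds multiplier-scaled score.
; It also slightly raises the player's walk speed within a clamped range, then destroys itself after a short delay.
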(event `self.ReceiveBeginPlay`
  (`self.SpawnObstacle`))

(event `self.Box.OnComponentBeginOverlap`
  (params (OverlappedComponent :type "PrimitiveComponent Object Reference") (OtherActor :type "Actor Object Reference") (OtherComp :type "PrimitiveComponent Object Reference") (OtherBodyIndex :type Integer) (bFromSweep :type Boolean) (SweepResult :type "HitResult Structure (by ref)"))
  (cast `/Game/EndlessRunner/Runner` OtherActor)
  (bind _asrunner_game_mode (cast `/Game/EndlessRunner/RunnerGameMode` (`GameplayStatics.GetGameMode`)))
  (`/Game/EndlessRunner/RunnerGameMode.SpawnTile` _asrunner_game_mode)
  (bind _asrunner_game_mode_2 (cast `/Game/EndlessRunner/RunnerGameMode` (`GameplayStatics.GetGameMode`)))
  (set `/Game/EndlessRunner/RunnerGameMode.CurrentScore` (+ (`/Game/EndlessRunner/RunnerGameMode.CurrentScore` _asrunner_game_mode_2) (* 1 (`/Game/EndlessRunner/RunnerGameMode.ScoreMultiplier` _asrunner_game_mode_2))) _asrunner_game_mode_2)
  (bind _asrunner (cast `/Game/EndlessRunner/Runner` (`GameplayStatics.GetPlayerCharacter` 0)))
  (bind _charactermovement (`Character.CharacterMovement` _asrunner))
  (set `CharacterMovementComponent.MaxWalkSpeed` (`KismetMathLibrary.FClamp` (* (`CharacterMovementComponent.MaxWalkSpeed` _charactermovement) 1.01) 600.0 2400.0) _charactermovement)
  (`KismetSystemLibrary.Delay` 1.0)
  (`self.K2_DestroyActor`))

(fn `SpawnObstacle`
  (`|ExecutionSequence`
    (:`then_0`
      (switch `int` (`KismetMathLibrary.RandomIntegerInRange` 0 2)
        (:`0`
          (`|SpawnActorFromClass` "/Game/EndlessRunner/Obstacle.Obstacle_C" (`SceneComponent.K2_GetComponentToWorld` (`self.LeftLane`)) "Undefined" "OverrideRootScale" null null))))
    (:`then_1`
      (switch `int` (`KismetMathLibrary.RandomIntegerInRange` 0 2)
        (:`1`
          (`|SpawnActorFromClass` "/Game/EndlessRunner/Obstacle.Obstacle_C" (`SceneComponent.K2_GetComponentToWorld` (`self.MiddleLane`)) "Undefined" "OverrideRootScale" null null))))
    (:`then_2`
      (switch `int` (`KismetMathLibrary.RandomIntegerInRange` 0 2)
        (:`2`
          (`|SpawnActorFromClass` "/Game/EndlessRunner/Obstacle.Obstacle_C" (`SceneComponent.K2_GetComponentToWorld` (`self.RightLane`)) "Undefined" "OverrideRootScale" null null))))))

(fn `UserConstructionScript`)